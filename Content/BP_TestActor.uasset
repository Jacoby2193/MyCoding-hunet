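; BP_TestActor is a scratch actor that exercises basic Blueprint scripting with loops, branches, variables and functions.
; On BeginPlay it loops over a small index range and prints the even indices below five to the screen.
; A MyAdd function returns the sum of two integers, but its only call sits in disconnected nodes.
; Other unwired experiments cover an in-air branch, a switch on Number and printing a name.
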(event `self.ReceiveBeginPlay`
  (for _index (range 10)
    (if (and (== (mod _index 2) 0) (< _index 5))
      (`KismetSystemLibrary.PrintString` (`KismetStringLibrary.Conv_IntToString` _index) true true (struct :`G` 0.66 :`B` 1.0 :`A` 1.0) 50.0))))

(event `self.ReceiveTick`
  (params (DeltaSeconds :type "Float (single-precision)")))

(fn `MyAdd`
  (params (A :type Integer) (B :type Integer))
  (returns (Result :type Integer))
  ;[1 1 1] 두 개의 정수를 더하는 기능
  (return (+ A B)))

(fn `UserConstructionScript`)